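; A score collectable that adds its ModifierValue to the player's score when something begins overlapping its capsule.
; The overlap handler updates PlayerScore on the GI_Main game instance, pushes the new total to the score widget referenced there, then destroys the actor.
; The overlap does not check which actor triggered it, and the construction script only calls its parent's version.
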(event `self.Capsule.OnComponentBeginOverlap`
  (params (OverlappedComponent :type "PrimitiveComponent Object Reference") (OtherActor :type "Actor Object Reference") (OtherComp :type "PrimitiveComponent Object Reference") (OtherBodyIndex :type Integer) (bFromSweep :type Boolean) (SweepResult :type "HitResult Structure (by ref)"))
  ; Collectable: Score Addition
  (bind _asgi_main (cast `/Game/MAIN/GI_Main` (`GameplayStatics.GetGameInstance`)))
  (bind _output_get (set `/Game/MAIN/GI_Main.PlayerScore` (+ (`/Game/MAIN/GI_Main.PlayerScore` _asgi_main) (`self.ModifierValue`)) _asgi_main))
  (`/Game/MAIN/Blueprints/Widgets/WBP_PlayerScore.ScoreUpdate` (`/Game/MAIN/GI_Main.ScoreWidgetRef` _asgi_main) _output_get)
  (`self.K2_DestroyActor`))

(fn `UserConstructionScript`
  (`parent.UserConstructionScript`))