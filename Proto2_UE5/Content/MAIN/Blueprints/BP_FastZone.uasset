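; BP_FastZone is a trigger zone that temporarily multiplies the player character's walk speed.
; On BeginPlay it caches the default MaxWalkSpeed; a Player-tagged overlap applies FastValue once, guarded by IsPlayerFast.
; Any end overlap, without a tag check, waits BoostDelay, then restores the cached speed and clears the flag.
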(event `self.ReceiveBeginPlay`
  (set `self.DefaultSpeed` (`CharacterMovementComponent.MaxWalkSpeed` (`Character.CharacterMovement` (`GameplayStatics.GetPlayerCharacter` 0)))))

(event `self.ReceiveActorBeginOverlap`
  (params (OtherActor :type "Actor Object Reference"))
  (bind _charactermovement (`Character.CharacterMovement` (`GameplayStatics.GetPlayerCharacter` 0)))
  (if (and (`self.ActorHasTag` OtherActor "Player") (not (`self.isPlayerFast`)))
    (set `CharacterMovementComponent.MaxWalkSpeed` (* (`CharacterMovementComponent.MaxWalkSpeed` _charactermovement) (`self.FastValue`)) _charactermovement)
    (set `self.isPlayerFast` true)))

(event `self.ReceiveActorEndOverlap`
  (params (OtherActor :type "Actor Object Reference"))
  (`KismetSystemLibrary.Delay` (`self.BoostDelay`))
  (set `CharacterMovementComponent.MaxWalkSpeed` (`self.DefaultSpeed`) (`Character.CharacterMovement` (`GameplayStatics.GetPlayerCharacter` 0)))
  (set `self.isPlayerFast` false))

(fn `UserConstructionScript`)