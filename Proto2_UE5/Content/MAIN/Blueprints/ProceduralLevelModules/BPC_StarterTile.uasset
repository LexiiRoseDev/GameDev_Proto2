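; Starter tile for procedural endless levels, which registers itself as the first module in GM_MainGameMode and generates two modules ahead on BeginPlay.
; StarterGeneration spawns a random module at the given module's Arrow using GI_Main's EndlessRandomStream, then inserts it at the front of the game mode's list.
; When that list overflows, it destroys the oldest module, updates the respawn and returns the new one for chaining.
; An older unrolled four-step generation chain remains unconnected.
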(event `self.ReceiveBeginPlay`
  ; Make self the first module
  (bind _asgm_main_game_mode (cast `/Game/MAIN/GM_MainGameMode` (`GameplayStatics.GetGameMode`)))
  (`KismetArrayLibrary.Array_Set` (`/Game/MAIN/GM_MainGameMode.LevelModules` _asgm_main_game_mode) 0 self)
  ; Generate 2 modules ahead
  (`KismetSystemLibrary.DelayUntilNextTick`)
  (bind _spawned_module (`self.StarterGeneration` self))
  (`self.StarterGeneration` _spawned_module))

(fn `StarterGeneration`
  (params (Object :type "Object Object Reference"))
  (returns (`Spawned Module` :type "/Game/MAIN/Blueprints/ProceduralLevelModules/BPP_LevelModule Object Reference"))
  (bind _levelmodules (`self.LevelModules`))
  (bind _asbpp_level_module (cast `/Game/MAIN/Blueprints/ProceduralLevelModules/BPP_LevelModule` Object))
  (bind _asgi_main (cast `/Game/MAIN/GI_Main` (`GameplayStatics.GetGameInstance`)))
  (bind _returnvalue (`|SpawnActorFromClass` (`|GetArrayItem` _levelmodules (`KismetMathLibrary.RandomIntegerInRangeFromStream` (`/Game/MAIN/GI_Main.Endless Random Stream` _asgi_main) 0 (- (`KismetArrayLibrary.Array_Length` _levelmodules) 1))) (`SceneComponent.K2_GetComponentToWorld` (`/Game/MAIN/Blueprints/ProceduralLevelModules/BPP_LevelModule.Arrow` _asbpp_level_module)) "AlwaysSpawn" "MultiplyWithRoot" null null))
  (`/Engine/EditorBlueprintResources/StandardMacros.IsValid` _returnvalue
    (:`Is Valid`
      _)
    (:`Is Not Valid`
      (`KismetSystemLibrary.PrintString` "But returned is invalid")))
  (bind _asgm_main_game_mode (cast `/Game/MAIN/GM_MainGameMode` (`GameplayStatics.GetGameMode`)))
  (bind _levelmodules_2 (`/Game/MAIN/GM_MainGameMode.LevelModules` _asgm_main_game_mode))
  (`KismetArrayLibrary.Array_Insert` _levelmodules_2 _returnvalue)
  (if (`KismetArrayLibrary.Array_IsValidIndex` _levelmodules_2 5)
    (bind _output (`|GetArrayItem` _levelmodules_2 5))
    (`/Engine/EditorBlueprintResources/StandardMacros.IsValid` _output
      (:`Is Valid`
        (`self.K2_DestroyActor` _output))
      (:`Is Not Valid`
        _))
    (`KismetArrayLibrary.Array_Remove` _levelmodules_2 5)
    (`/Engine/EditorBlueprintResources/StandardMacros.IsValid` _returnvalue
      (:`Is Valid`
        _)
      (:`Is Not Valid`
        (`KismetSystemLibrary.PrintString` " Gen Invalid")))
    (`/Game/MAIN/GM_MainGameMode.SetNewRespawn` _asgm_main_game_mode)
    (return _returnvalue)
    (else
      (`KismetSystemLibrary.PrintString` "Invalid Index"))))

(fn `UserConstructionScript`
  (`parent.UserConstructionScript`))