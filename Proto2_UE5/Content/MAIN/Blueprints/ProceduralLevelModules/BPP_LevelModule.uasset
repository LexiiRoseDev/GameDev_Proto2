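; Procedural level module that chains randomly chosen modules ahead of the player for an endless-style run.
; Player overlap with a one-shot trigger makes the front module spawn another at its Arrow, keeping a five-module rolling list in GM_MainGameMode.
; The oldest module becomes the respawn point and activates its death wall.
; Death box or active wall hits teleport the player there, subtract 30 seconds from total time and briefly disable input.
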(event `self.SpawnNewModuleCollision.OnComponentBeginOverlap`
  (params (OverlappedComponent :type "PrimitiveComponent Object Reference") (OtherActor :type "Actor Object Reference") (OtherComp :type "PrimitiveComponent Object Reference") (OtherBodyIndex :type Integer) (bFromSweep :type Boolean) (SweepResult :type "HitResult Structure (by ref)"))
  ; Spawn Module At Front
  (if (== OtherActor (`GameplayStatics.GetPlayerPawn` 0))
    (bind _asgm_main_game_mode (cast `/Game/MAIN/GM_MainGameMode` (`GameplayStatics.GetGameMode`)))
    (`self.GenerateNewRoom` (`|GetArrayItem` (`/Game/MAIN/GM_MainGameMode.LevelModules` _asgm_main_game_mode))) ; Generate new module from front module
    (`ActorComponent.K2_DestroyComponent` (`self.SpawnNewModuleCollision`)) ; Destroy Collision box to \neliminate repeated activation
    (bind _output (`|GetArrayItem` (`/Game/MAIN/GM_MainGameMode.LevelModules` _asgm_main_game_mode) 4))
    (`/Engine/EditorBlueprintResources/StandardMacros.IsValid` _output
      (:`Is Valid`
        (`SceneComponent.SetVisibility` (`/Game/MAIN/Blueprints/ProceduralLevelModules/BPP_LevelModule.DeathWall` _output) true false)
        (set `/Game/MAIN/Blueprints/ProceduralLevelModules/BPP_LevelModule.DeathWallActive` true _output)))))

(event `self.DeathBox.OnComponentBeginOverlap`
  (params (OverlappedComponent :type "PrimitiveComponent Object Reference") (OtherActor :type "Actor Object Reference") (OtherComp :type "PrimitiveComponent Object Reference") (OtherBodyIndex :type Integer) (bFromSweep :type Boolean) (SweepResult :type "HitResult Structure (by ref)"))
  (bind _returnvalue (`GameplayStatics.GetPlayerCharacter` 0))
  (bind _returnvalue_2 (`GameplayStatics.GetPlayerController` 0))
  ; Death Box Functionality
  (set `self.Other Actor` OtherActor)
  (if (`self.ActorHasTag` OtherActor "Player")
    (`KismetSystemLibrary.PrintString` "The chosen one has fallen." :!label _label)
    (bind _asgi_main (cast `/Game/MAIN/GI_Main` (`GameplayStatics.GetGameInstance`))
      (:`then`
        (`self.K2_SetActorTransform` (`self.Other Actor`) (`/Game/MAIN/GI_Main.Respawn` _asgi_main) false false)
        (set `/Game/MAIN/GI_Main.PlayerTotalTime` (- (`/Game/MAIN/GI_Main.PlayerTotalTime` _asgi_main) 30) _asgi_main)
        (`KismetSystemLibrary.PrintString` "-30 Seconds" true true (struct :`R` 0.711458 :`G` 0.008871 :`A` 1.0) 5.0)
        (`/Game/MAIN/Blueprints/Widgets/WBP_Timer.UpdateTimer` (`/Game/MAIN/GI_Main.Timer Widget` _asgi_main))
        (`self.DisableInput` _returnvalue _returnvalue_2)
        (`KismetSystemLibrary.Delay` 0.5)
        (`self.EnableInput` _returnvalue _returnvalue_2))
      (:`CastFailed`
        (`KismetSystemLibrary.PrintString` "Respawn Failed")))))

(event `self.DeathWall.OnComponentBeginOverlap`
  (params (OverlappedComponent :type "PrimitiveComponent Object Reference") (OtherActor :type "Actor Object Reference") (OtherComp :type "PrimitiveComponent Object Reference") (OtherBodyIndex :type Integer) (bFromSweep :type Boolean) (SweepResult :type "HitResult Structure (by ref)"))
  (set `self.Other Actor` OtherActor)
  (if (`self.ActorHasTag` OtherActor "Player")
    (if (`self.DeathWallActive`)
      (goto _label))))

(fn `GenerateNewRoom`
  (returns (`Generated Room` :type "/Game/MAIN/Blueprints/ProceduralLevelModules/BPP_LevelModule Object Reference"))
  (bind _levelmodules (`self.LevelModules`))
  (bind _returnvalue (`|SpawnActorFromClass` (`|GetArrayItem` _levelmodules (`KismetMathLibrary.RandomIntegerInRange` 0 (- (`KismetArrayLibrary.Array_Length` _levelmodules) 1))) (`SceneComponent.K2_GetComponentToWorld` (`self.Arrow`)) "AlwaysSpawn" "MultiplyWithRoot" null null))
  (`/Engine/EditorBlueprintResources/StandardMacros.IsValid` _returnvalue
    (:`Is Valid`
      (bind _asgm_main_game_mode (cast `/Game/MAIN/GM_MainGameMode` (`GameplayStatics.GetGameMode`)))
      (bind _levelmodules_2 (`/Game/MAIN/GM_MainGameMode.LevelModules` _asgm_main_game_mode))
      (`KismetArrayLibrary.Array_Insert` _levelmodules_2 _returnvalue)
      (if (`KismetArrayLibrary.Array_IsValidIndex` _levelmodules_2 5)
        (bind _output (`|GetArrayItem` _levelmodules_2 5))
        (`/Engine/EditorBlueprintResources/StandardMacros.IsValid` _output
          (:`Is Valid`
            (`self.K2_DestroyActor` _output))
          (:`Is Not Valid`
            _))
        (`KismetArrayLibrary.Array_Remove` _levelmodules_2 5)
        (else
          (`KismetSystemLibrary.PrintString` "Invalid Index")))
      (`/Engine/EditorBlueprintResources/StandardMacros.IsValid` _returnvalue
        (:`Is Valid`
          _)
        (:`Is Not Valid`
          (`KismetSystemLibrary.PrintString` " Gen Invalid")))
      (bind _asgm_main_game_mode_2 (cast `/Game/MAIN/GM_MainGameMode` (`GameplayStatics.GetGameMode`)))
      (bind _output_2 (`|GetArrayItem` (`/Game/MAIN/GM_MainGameMode.LevelModules` _asgm_main_game_mode_2) 4))
      (`/Engine/EditorBlueprintResources/StandardMacros.IsValid` _output_2
        (:`Is Valid`
          (bind _asgi_main (cast `/Game/MAIN/GI_Main` (`GameplayStatics.GetGameInstance`)))
          (set `/Game/MAIN/GI_Main.Respawn` (`SceneComponent.K2_GetComponentToWorld` (`/Game/MAIN/Blueprints/ProceduralLevelModules/BPP_LevelModule.RespawnPoint` _output_2)) _asgi_main)
          (return _returnvalue))))))

(fn `UserConstructionScript`)