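; A procedural level module that offers a time-bonus collectable and a score collectable, apparently as an either/or pickup for the player.
; On BeginPlay it spawns both at its two spawn points.
; Player overlap with the top trigger box destroys the score collectable, while the bottom box destroys the time one.
; Either trigger then removes both boxes, so only the first overlap counts.
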(event `self.ReceiveBeginPlay`
  (bind _returnvalue (`|SpawnActorFromClass` "/Game/MAIN/Blueprints/Collectables/BPC_CollectableAddTime.BPC_CollectableAddTime_C" (`SceneComponent.K2_GetComponentToWorld` (`self.CollectableSP1`)) "Undefined" "MultiplyWithRoot" null null))
  (bind _returnvalue_2 (`|SpawnActorFromClass` "/Game/MAIN/Blueprints/Collectables/BPP_CollectableAddScore.BPP_CollectableAddScore_C" (`SceneComponent.K2_GetComponentToWorld` (`self.CollectableSP2`)) "Undefined" "MultiplyWithRoot" null null)))

(event `self.BoxColTop.OnComponentBeginOverlap`
  (params (OverlappedComponent :type "PrimitiveComponent Object Reference") (OtherActor :type "Actor Object Reference") (OtherComp :type "PrimitiveComponent Object Reference") (OtherBodyIndex :type Integer) (bFromSweep :type Boolean) (SweepResult :type "HitResult Structure (by ref)"))
  (if (`self.ActorHasTag` OtherActor "Player")
    (`self.K2_DestroyActor` (stale `self.ReceiveBeginPlay` _returnvalue_2))
    (`ActorComponent.K2_DestroyComponent` (`self.BoxColBottom`))
    (`ActorComponent.K2_DestroyComponent` (`self.BoxColTop`))))

(event `self.BoxColBottom.OnComponentBeginOverlap`
  (params (OverlappedComponent :type "PrimitiveComponent Object Reference") (OtherActor :type "Actor Object Reference") (OtherComp :type "PrimitiveComponent Object Reference") (OtherBodyIndex :type Integer) (bFromSweep :type Boolean) (SweepResult :type "HitResult Structure (by ref)"))
  (if (`self.ActorHasTag` OtherActor "Player")
    (`self.K2_DestroyActor` (stale `self.ReceiveBeginPlay` _returnvalue))
    (`ActorComponent.K2_DestroyComponent` (`self.BoxColBottom`))
    (`ActorComponent.K2_DestroyComponent` (`self.BoxColTop`))))

(fn `UserConstructionScript`
  (`parent.UserConstructionScript`))