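; BP_Deathbox is a kill volume that sends the player back to a saved respawn point.
; On actor overlap it checks for the "Player" tag, then moves that actor to the Respawn transform stored in GI_Main, the game instance.
; It prints debug messages for the fall, the player's total time and a failed cast; a 30-unit time penalty exists but is not connected.
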(event `self.ReceiveActorBeginOverlap`
  (params (OtherActor :type "Actor Object Reference"))
  (set `self.Other Actor` OtherActor)
  (if (`self.ActorHasTag` OtherActor "Player")
    (`KismetSystemLibrary.PrintString` "The chosen one has fallen.")
    (bind _asgi_main (cast `/Game/MAIN/GI_Main` (`GameplayStatics.GetGameInstance`))
      (:`then`
        (`self.K2_SetActorTransform` (`self.Other Actor`) (`/Game/MAIN/GI_Main.Respawn` _asgi_main) false false)
        (`KismetSystemLibrary.PrintString` (`KismetStringLibrary.Conv_IntToString` (`/Game/MAIN/GI_Main.PlayerTotalTime` _asgi_main))))
      (:`CastFailed`
        (`KismetSystemLibrary.PrintString` "Respawn Failed")))))

(fn `UserConstructionScript`)