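; BP_SlowZone is a zone actor that slows the player while they are inside it and for a short time after.
; Overlap by a "Player"-tagged actor multiplies player 0's MaxWalkSpeed by SlowValue once, guarded by IsPlayerSlow.
; Exit waits SlowDelay, then restores the speed cached at BeginPlay, even if the player has re-entered.
; Both transitions print debug strings.
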(event `self.ReceiveBeginPlay`
  (set `self.DefaultSpeed` (`CharacterMovementComponent.MaxWalkSpeed` (`Character.CharacterMovement` (`GameplayStatics.GetPlayerCharacter` 0)))))

(event `self.ReceiveActorBeginOverlap`
  (params (OtherActor :type "Actor Object Reference"))
  (bind _charactermovement (`Character.CharacterMovement` (`GameplayStatics.GetPlayerCharacter` 0)))
  (if (and (`self.ActorHasTag` OtherActor "Player") (not (`self.isPlayerSlow`)))
    (`KismetSystemLibrary.PrintString` "player slow")
    (set `CharacterMovementComponent.MaxWalkSpeed` (* (`CharacterMovementComponent.MaxWalkSpeed` _charactermovement) (`self.SlowValue`)) _charactermovement)
    (set `self.isPlayerSlow` true)))

(event `self.ReceiveActorEndOverlap`
  (params (OtherActor :type "Actor Object Reference"))
  (if (`self.ActorHasTag` OtherActor "Player")
    (set `self.isOverlap` false)
    (`KismetSystemLibrary.Delay` (`self.SlowDelay`))
    (`KismetSystemLibrary.PrintString` "Player no slow")
    (set `CharacterMovementComponent.MaxWalkSpeed` (`self.DefaultSpeed`) (`Character.CharacterMovement` (`GameplayStatics.GetPlayerCharacter` 0)))
    (set `self.isPlayerSlow` false)))

(fn `UserConstructionScript`)